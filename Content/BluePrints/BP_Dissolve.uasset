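; BP_Dissolve is an actor whose static mesh changes through a dissolve material parameter and loses collision when something overlaps it.
; BeginPlay creates a dynamic material instance from the mesh's first material slot.
; Begin overlap plays a timeline and end overlap reverses it, with each update writing the "Amount" scalar.
; The same update sets collision from timeline direction: disabled while playing forward, query and physics while reversing.
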(event `self.ReceiveBeginPlay`
  (bind _returnvalue (`KismetMaterialLibrary.CreateDynamicMaterialInstance` (`PrimitiveComponent.GetMaterial` (`self.StaticMeshComponent`) 0) "None"))
  (bind _output_get (set `self.DynamicMertirial` _returnvalue))
  (`PrimitiveComponent.SetMaterial` (`self.StaticMeshComponent`) 0 _output_get))

(event `self.ReceiveActorBeginOverlap`
  (params (OtherActor :type "Actor Object Reference"))
  (bind (_direction _output) (`Timeline|Timeline` :!label _label)
    (:`Update`
      (`MaterialInstanceDynamic.SetScalarParameterValue` (`self.DynamicMertirial`) "Amount" _output)
      (`PrimitiveComponent.SetCollisionEnabled` (`self.StaticMeshComponent`) (select `bool` (`|EnumEquality` _direction "Forward") :`false` "QueryAndPhysics" :`true` "NoCollision" :!type "ECollisionEnabled Enum")))))

(event `self.ReceiveActorEndOverlap`
  (params (OtherActor :type "Actor Object Reference"))
  (goto _label :!via `Reverse`))

(fn `UserConstructionScript`)