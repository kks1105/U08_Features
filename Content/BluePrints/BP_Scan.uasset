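; BP_Scan is an overlap-triggered scan effect that drives a post-process through the CBuffer_Scan material parameter collection.
; An actor overlap enables the PostProcess component and replays a timeline at a slowed rate, writing its output to the Clock parameter.
; Tick continuously writes the player character's location to the PlayerPosition parameter.
; The post-process starts disabled in the construction script and is disabled again when an overlap ends.
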(event `self.ReceiveActorBeginOverlap`
  (params (OtherActor :type "Actor Object Reference"))
  (set `PostProcessComponent.bEnabled` true (`self.PostProcess`))
  (`TimelineComponent.SetPlayRate` (`self.timeline`) 0.1)
  (bind (_direction _output) (`Timeline|timeline` :!via `PlayFromStart`)
    (:`Update`
      (`KismetMaterialLibrary.SetScalarParameterValue` "/Game/PostProsses/CBuffer_Scan.CBuffer_Scan" "Clock" _output))))

(event `self.ReceiveActorEndOverlap`
  (params (OtherActor :type "Actor Object Reference"))
  (set `PostProcessComponent.bEnabled` false (`self.PostProcess`)))

(event `self.ReceiveTick`
  (params (DeltaSeconds :type "Float (single-precision)"))
  (`KismetMaterialLibrary.SetVectorParameterValue` "/Game/PostProsses/CBuffer_Scan.CBuffer_Scan" "PlayerPosition" (`KismetMathLibrary.Conv_VectorToLinearColor` (`self.K2_GetActorLocation` (`GameplayStatics.GetPlayerCharacter` 0)))))

(fn `UserConstructionScript`
  (set `PostProcessComponent.bEnabled` false (`self.PostProcess`)))